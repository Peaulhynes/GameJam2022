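; BP_Zone is a shrinking zone actor, in the style of a battle royale safe area, that scales down in steps.
; Timed breaks alternate with shrink phases, where Tick eases the actor scale between consecutive step values using per-step durations.
; It exposes the collision sphere's radius and current step damage, but character overlaps only print debug messages, applying no damage.
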(event `ShrinkOver`
  (set `self.Timer` 0.0)
  (set `self.Action` "NewEnumerator1")
  (bind _output_get (set `self.Step` (+ (`self.Step`) 1)))
  (if (< _output_get (- (`KismetArrayLibrary.Array_Length` (`self.StepsScales`)) 1))
    (`KismetSystemLibrary.K2_SetTimerDelegate` (delegate `BreakOver`) (`|GetArrayItem` (`self.BreakTimes`) (`self.Step`)) :!label _label)))

(event `BreakOver`
  (set `self.Timer` 0.0)
  (set `self.Action` "NewEnumerator0"))

(event `self.ReceiveBeginPlay`
  (`self.SetActorScale3D` (`KismetMathLibrary.Conv_DoubleToVector` (`|GetArrayItem` (`self.StepsScales`))))
  (set `PrimitiveComponent.bGenerateOverlapEvents` true (`self.ZoneCollision`))
  (goto _label))

(event `self.ReceiveTick`
  (params (DeltaSeconds :type "Float (single-precision)"))
  (bind _stepsscales (`self.StepsScales`))
  (bind _step (`self.Step`))
  (bind _output_get (set `self.Timer` (+ (`self.Timer`) DeltaSeconds)))
  (if (`|EnumEquality` (`self.Action`) "NewEnumerator0")
    (bind _returnvalue (/ _output_get (`|GetArrayItem` (`self.ShrinkTimes`) _step)))
    (if (>= _returnvalue 0.9999)
      (`self.ShrinkOver`)
      (else
        (`self.SetActorScale3D` (`KismetMathLibrary.Conv_DoubleToVector` (`|EaseFunction` "EaseOut" (`KismetMathLibrary.FClamp` _returnvalue) (`|GetArrayItem` _stepsscales _step) (`|GetArrayItem` _stepsscales (+ _step 1)))))))))

(event `self.ReceiveActorBeginOverlap`
  (params (OtherActor :type "Actor Object Reference"))
  (cast `/Game/ThirdPersonCPP/Blueprints/ThirdPersonCharacter` OtherActor)
  (`KismetSystemLibrary.PrintString` "BeginOverlap Zone"))

(event `self.ReceiveActorEndOverlap`
  (params (OtherActor :type "Actor Object Reference"))
  (cast `/Game/ThirdPersonCPP/Blueprints/ThirdPersonCharacter` OtherActor)
  (bind _damages (`self.GetCurrentStepDamages`))
  (`KismetSystemLibrary.PrintString` (`KismetStringLibrary.Concat_StrStr` "EndOverlap Zone; Damages: " (`KismetStringLibrary.Conv_DoubleToString` _damages))))

(fn `GetCurrentStepDamages`
  (returns (Damages :type "Float (double-precision)"))
  (return (`|GetArrayItem` (`self.StepsDamages`) (`self.Step`))))

(fn `GetRadius`
  (returns (Radius :type "Float (double-precision)"))
  (return (`SphereComponent.GetScaledSphereRadius` (`self.ZoneCollision`))))

(fn `UserConstructionScript`)