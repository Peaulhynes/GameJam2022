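; Game mode that periodically rolls a random difficulty level on a resource spawn timer.
; Tick accumulates time and, while the map's resource count is under its maximum, resets the timer and rolls once the spawn interval elapses.
; The roll is a weighted pick over DifficultyLevels by SpawnFrequency, printing and returning the chosen entry.
; Tick ignores the result, and no actual spawning happens here.
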(event `self.ReceiveBeginPlay`)

(event `self.ReceiveTick`
  (params (DeltaSeconds :type "Float (single-precision)"))
  (set `self.Timer` (+ DeltaSeconds (`self.Timer`)))
  (if (< (`self.ResourcesOnMap`) (`self.MaxResourcesOnMap`))
    (if (>= (`self.Timer`) (`self.SpawnInterval`))
      (set `self.Timer` 0.0)
      (`self.GetRandomDifficultyLevel`))))

(fn `GetRandomDifficultyLevel`
  (returns (Level :type "/Game/Structs/FDifficultyLevel Structure"))
  (locals (Weight :type "Float (double-precision)") (Rand :type "Float (double-precision)" :default 0.0))
  (bind _weight (`local.Weight`))
  (set `local.Weight` 0.0)
  (for _array_element (`self.DifficultyLevels`)
    (set `local.Weight` (+ (`.SpawnFrequency_17_812554534C6E8035D9E0BFA140FAC3D2` (break `/Game/Structs/FDifficultyLevel` _array_element)) _weight)))
  (set `local.Rand` (`KismetMathLibrary.RandomFloatInRange` 0.0 _weight))
  (for _array_element_2 (`self.DifficultyLevels`)
    (bind (_difficulty _centerdistancemin _centerdistancemax _spawnfrequency) (break `/Game/Structs/FDifficultyLevel` _array_element_2))
    (set `local.Rand` (- (`local.Rand`) _spawnfrequency))
    (if (<= (`local.Rand`) 0.0)
      (`|ExecutionSequence`
        (:`then_0`
          (break))
        (:`then_1`
          (`KismetSystemLibrary.PrintString` (`|GetEnumeratorNameAsString` _difficulty))
          (return _array_element_2))))))

(fn `UserConstructionScript`)