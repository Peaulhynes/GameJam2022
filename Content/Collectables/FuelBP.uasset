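; Fuel collectable that adds one Fuel to the player's ThirdPersonCharacter on overlap, then destroys itself.
; Each pickup recalculates MaxWalkSpeed by linear interpolation, slowing the character from MaxSpeed toward MinSpeed as Fuel approaches MaxFuel.
; It prints the new speed to screen and disables shadow casting on its Widget component at BeginPlay.
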(event `self.ReceiveBeginPlay`
  (`PrimitiveComponent.SetCastShadow` (`self.Widget`) false))

(event `self.ReceiveActorBeginOverlap`
  (params (OtherActor :type "Actor Object Reference"))
  (bind _returnvalue (`GameplayStatics.GetPlayerPawn` 0))
  (if (== OtherActor _returnvalue)
    (bind _asthird_person_character (cast `/Game/ThirdPersonCPP/Blueprints/ThirdPersonCharacter` _returnvalue))
    (`/Engine/EditorBlueprintResources/StandardMacros.IncrementFloat` (`/Game/ThirdPersonCPP/Blueprints/ThirdPersonCharacter.Fuel` _asthird_person_character)
      (:`  `
        (bind _minspeed (`/Game/ThirdPersonCPP/Blueprints/ThirdPersonCharacter.MinSpeed` _asthird_person_character))
        (bind _returnvalue_2 (+ (* (- (`/Game/ThirdPersonCPP/Blueprints/ThirdPersonCharacter.MaxSpeed` _asthird_person_character) _minspeed) (- 1.0 (/ (/ (* (`/Game/ThirdPersonCPP/Blueprints/ThirdPersonCharacter.Fuel` _asthird_person_character) 100.0) (`/Game/ThirdPersonCPP/Blueprints/ThirdPersonCharacter.MaxFuel` _asthird_person_character)) 100.0))) _minspeed))
        (set `CharacterMovementComponent.MaxWalkSpeed` _returnvalue_2 (`Character.CharacterMovement` _asthird_person_character))
        (`self.K2_DestroyActor`)
        (`KismetSystemLibrary.PrintString` (`KismetStringLibrary.Conv_DoubleToString` _returnvalue_2))))))

(fn `UserConstructionScript`)