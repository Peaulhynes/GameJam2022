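; Actor component that makes its owning actor fall at a constant speed until it lands on something.
; BeginPlay sets OnGround from a short downward Visibility line trace, then calls TouchedGround whatever the result.
; While not grounded, Tick sweeps the owner downward, and a blocking hit sets OnGround and calls TouchedGround again.
; The ground trace leaves persistent debug drawing and prints on a hit.
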(event `self.ReceiveBeginPlay`
  (bind _onground (`self.IsOnGround`))
  (set `self.OnGround` _onground)
  (`self.TouchedGround`))

(event `self.ReceiveTick`
  (params (DeltaSeconds :type "Float (single-precision)"))
  (bind _returnvalue (`self.GetOwner`))
  (if (not (`self.OnGround`))
    (bind _sweephitresult (`Actor.K2_SetActorLocation` _returnvalue (- (`Actor.K2_GetActorLocation` _returnvalue) (`KismetMathLibrary.MakeVector` 0.0 0.0 (* DeltaSeconds (`self.FallingSpeed`)))) true false))
    (if (`GameplayStatics.BreakHitResult` _sweephitresult)
      (set `self.OnGround` true)
      (`self.TouchedGround`))))

(fn `IsOnGround`
  (returns (OnGround :type Boolean))
  (bind _returnvalue (`self.GetOwner`))
  (bind _returnvalue_2 (`Actor.K2_GetActorLocation` _returnvalue))
  (bind (_outhit _returnvalue_3) (`KismetSystemLibrary.LineTraceSingle` _returnvalue_2 (- _returnvalue_2 (`KismetMathLibrary.MakeVector` 0.0 0.0 (`self.GroundLineSize`))) "TraceTypeQuery1" false (`|MakeArray` _returnvalue) "Persistent"))
  (if _returnvalue_3
    (if (`GameplayStatics.BreakHitResult` _outhit)
      (`KismetSystemLibrary.PrintString` "onGround" true true (struct :`G` 0.66 :`B` 1.0 :`A` 1.0) 0.0)
      (return true)
      (else
        (return false)))))