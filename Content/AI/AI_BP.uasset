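; AI_BP is an enemy that chases the player, drains their fuel at close range and dies when shot.
; PawnSensing triggers an AI MoveTo toward the player pawn when it is seen.
; DrainSphere overlap sets an in-range flag and runs a delayed loop that periodically lowers ThirdPersonCharacter Fuel while it is above zero.
; A Projectile overlapping the capsule destroys both the enemy and the projectile.
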(event `self.DrainSphere.OnComponentBeginOverlap`
  (params (OverlappedComponent :type "PrimitiveComponent Object Reference") (OtherActor :type "Actor Object Reference") (OtherComp :type "PrimitiveComponent Object Reference") (OtherBodyIndex :type Integer) (bFromSweep :type Boolean) (SweepResult :type "HitResult Structure (by ref)"))
  (bind _returnvalue (`GameplayStatics.GetPlayerCharacter` 0))
  ;[1 1 1] Drain Mechanic
  (if (== OtherActor _returnvalue)
    (bind _output_get (set `self.isInRange` true))
    (if _output_get :!label _label
      (bind _asthird_person_character (cast `/Game/ThirdPersonCPP/Blueprints/ThirdPersonCharacter` _returnvalue))
      (bind _fuel (`/Game/ThirdPersonCPP/Blueprints/ThirdPersonCharacter.Fuel` _asthird_person_character))
      (if (not (<= _fuel 0.0))
        (set `/Game/ThirdPersonCPP/Blueprints/ThirdPersonCharacter.Fuel` (- _fuel 0.5) _asthird_person_character))
      (`KismetSystemLibrary.Delay` 1.5)
      (goto _label))))

(event `self.DrainSphere.OnComponentEndOverlap`
  (params (OverlappedComponent :type "PrimitiveComponent Object Reference") (OtherActor :type "Actor Object Reference") (OtherComp :type "PrimitiveComponent Object Reference") (OtherBodyIndex :type Integer))
  ;[1 1 1] Drain Mechanic
  (if (== OtherActor (`GameplayStatics.GetPlayerCharacter` 0))
    (set `self.isInRange` false)))

(event `self.PawnSensing.OnSeePawn`
  (params (Pawn :type "Pawn Object Reference"))
  (bind _returnvalue (`GameplayStatics.GetPlayerPawn` 0))
  ;[1 1 1] Sense
  (if (== Pawn _returnvalue)
    (`|AIMoveTo` self (0.0 0.0 0.0) _returnvalue)))

(event `self.CapsuleComponent.OnComponentBeginOverlap`
  (params (OverlappedComponent :type "PrimitiveComponent Object Reference") (OtherActor :type "Actor Object Reference") (OtherComp :type "PrimitiveComponent Object Reference") (OtherBodyIndex :type Integer) (bFromSweep :type Boolean) (SweepResult :type "HitResult Structure (by ref)"))
  (bind _asprojectile (cast `/Game/ThirdPersonCPP/Blueprints/Projectile` OtherActor))
  (if (== OtherActor _asprojectile)
    (`self.K2_DestroyActor`)
    (`self.K2_DestroyActor` _asprojectile)))

(fn `UserConstructionScript`)